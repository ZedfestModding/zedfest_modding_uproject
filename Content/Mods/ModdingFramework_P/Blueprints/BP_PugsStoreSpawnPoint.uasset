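; Modding-framework store spawn marker that spawns a BP_StoreSpawnPoint at its transform, hides itself in game and advances a wave count when stores arrive.
; While it has no valid wave counter, Tick finds an existing BP_WaveCounter or spawns one.
; Cube overlaps wait three seconds, then each BP_Store not already recorded is added to a list and increments the counter's current wave number.
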(event OnComponentBeginOverlap(Cube)
  (params (OverlappedComponent :type Primitive%20Component%20Object%20Reference) (OtherActor :type Actor%20Object%20Reference) (OtherComp :type Primitive%20Component%20Object%20Reference) (OtherBodyIndex :type Integer) (bFromSweep :type Boolean) (SweepResult :type Hit%20Result%20Structure%20%28by%20ref%29))
  (bind _wavecounter (Variables|Default|GetWaveCounter))
  (Utilities|FlowControl|Delay 3.0)
  (bind _asbp_store (Utilities|Casting|CastToBP_Store OtherActor))
  (Variables|Default|SetBP_Store _asbp_store)
  (if (not (Utilities|Array|ContainsItem (Variables|Default|GetBP_Stores) (Variables|Default|GetBP_Store)))
    (Utilities|Array|Add (Variables|Default|GetBP_Stores) 0)
    (Variables|/Game/Mods/ModdingFramework_P/Blueprints/BP_WaveCounter.BP_WaveCounter_C|SetCurrentWaveNumber _wavecounter (+ 1 (Variables|/Game/Mods/ModdingFramework_P/Blueprints/BP_WaveCounter.BP_WaveCounter_C|GetCurrentWaveNumber _wavecounter)))))

(event EventBeginPlay
  (Game|SpawnActorfromClass "/Game/Blueprints/BP_StoreSpawnPoint.BP_StoreSpawnPoint_C" (Transformation|GetActorTransform) "AlwaysSpawn" 0 0)
  (Rendering|SetActorHiddenInGame true))

(event EventTick
  (params (DeltaSeconds :type Float%20%28single-precision%29))
  (Variables|Default|GetWaveCounter
    (:then)
    (:else
      (bind _outactors (Actor|GetAllActorsOfClass "/Game/Mods/ModdingFramework_P/Blueprints/BP_WaveCounter.BP_WaveCounter_C"))
      (Variables|Default|SetWaveCounters _outactors)
      (if (== 0 (Utilities|Array|Length (Variables|Default|GetWaveCounters)))
        (bind _returnvalue (Game|SpawnActorfromClass "/Game/Mods/ModdingFramework_P/Blueprints/BP_WaveCounter.BP_WaveCounter_C" (Math|Transform|MakeTransform "0, 0, 0" "0, 0, 0" "1,1,1") "AdjustIfPossibleButAlwaysSpawn" 0 0))
        (Variables|Default|SetWaveCounter _returnvalue)
        (else
          (Variables|Default|SetWaveCounter (Utilities|Array|Get(acopy) (Variables|Default|GetWaveCounters))))))))

(fn ConstructionScript)