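; Modding framework actor that reports the current horde difficulty when something overlaps its Plane component.
; The Plane is hidden in game on BeginPlay and acts as an invisible trigger.
; On overlap it reads CurrentDifficulty from BP_Horde_Gamestate and passes the matching name, Scrub through Impossible, to the PrintToModLoader event, which has an empty body here.
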(event OnComponentBeginOverlap(Plane)
  (params (OverlappedComponent :type Primitive%20Component%20Object%20Reference) (OtherActor :type Actor%20Object%20Reference) (OtherComp :type Primitive%20Component%20Object%20Reference) (OtherBodyIndex :type Integer) (bFromSweep :type Boolean) (SweepResult :type Hit%20Result%20Structure%20%28by%20ref%29))
  (Variables|Default|SetDifficulty (Variables|/Game/HordeTemplateBP/Blueprint/Base/BP_Horde_Gamestate.BP_Horde_Gamestate_C|GetCurrentDifficulty (.AsBP%20Horde%20Gamestate (Utilities|Casting|CastToBP_Horde_Gamestate (Game|GetGameState)))))
  (if (== 1 (Variables|Default|GetDifficulty))
    (CallFunction|PrinttoModLoader "Difficulty is Scrub")
    (elif (== 2 (Variables|Default|GetDifficulty))
      (CallFunction|PrinttoModLoader "Difficulty is Normal")
      (elif (== 3 (Variables|Default|GetDifficulty))
        (CallFunction|PrinttoModLoader "Difficulty is Hardcore")
        (elif (== 4 (Variables|Default|GetDifficulty))
          (CallFunction|PrinttoModLoader "Difficulty is Kamikaze")
          (elif (== 5 (Variables|Default|GetDifficulty))
            (CallFunction|PrinttoModLoader "Difficulty is Impossible")))))))

(event Custom|PrintToModLoader
  (params (Message :type String)))

(event EventBeginPlay
  (Development|SetHiddeninGame (Variables|Default|GetPlane) true false))

(fn ConstructionScript)