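; Modding-framework actor that reskins player pawns by replacing their skeletal meshes with MR_Ticklehead in solid M_Black material.
; One second after BeginPlay, it hides its Plane component and gathers every BP_Pawn in the level.
; Each skeletal mesh component on those pawns gets the new mesh with a pose reset, then M_Black on every material slot.
; The swap runs once, so pawns spawned later are untouched.
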(event EventBeginPlay
  (Utilities|FlowControl|Delay 1.0)
  (Development|SetHiddeninGame (Variables|Default|GetPlane) true false)
  (bind _outactors (Actor|GetAllActorsOfClass "/Game/NetworkRagdollIK/Blueprints/BP_Pawn.BP_Pawn_C"))
  (for _array_element _outactors
    (for _array_element_2 (Actor|GetComponentsByClass _array_element "/Script/Engine.SkeletalMeshComponent")
      (Class|SkinnedMeshComponent|SetSkeletalMesh _array_element_2 "/Game/Characters/Funny_Robot/Mesh/MR_Ticklehead.MR_Ticklehead" true)
      (for (_ _array_index) (Rendering|Material|GetMaterials _array_element_2)
        (Rendering|Material|SetMaterial _array_element_2 _array_index "/Game/Mods/ModdingFramework_P/Materials/M_Black.M_Black")))))

(fn ConstructionScript)