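; Modding framework trigger actor that attaches a megaphone static mesh to whatever actor overlaps its plane, intended for the player by its name.
; The plane is hidden on BeginPlay and serves as the overlap trigger.
; Each overlap spawns an actor, adds a scaled-down, collision-free mesh component at runtime, and snaps it to the overlapping actor.
; The overlap is not filtered to players or limited to one attachment.
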(event OnComponentBeginOverlap(Plane)
  (params (OverlappedComponent :type Primitive%20Component%20Object%20Reference) (OtherActor :type Actor%20Object%20Reference) (OtherComp :type Primitive%20Component%20Object%20Reference) (OtherBodyIndex :type Integer) (bFromSweep :type Boolean) (SweepResult :type Hit%20Result%20Structure%20%28by%20ref%29))
  (Variables|Default|SetOverlapped%20Actor OtherActor)
  (bind _returnvalue (Game|SpawnActorfromClass "/Script/Engine.Actor" (Math|Transform|MakeTransform "0, 0, 0" "0, 0, 0" "1.000000,1.000000,1.000000") "AdjustIfPossibleButAlwaysSpawn" 0 0))
  (Variables|Default|SetSpawnedActor _returnvalue)
  (bind _returnvalue_2 (AddComponent|AddStaticMeshComponent (Variables|Default|GetSpawnedActor) false))
  (bind _output_get (Variables|Default|SetMeshComponent _returnvalue_2))
  (Transformation|SetRelativeScale3D _output_get (* (Variables|/Script/Engine.SceneComponent|GetRelativeScale3D _output_get) 0.25))
  (Collision|SetCollisionEnabled (Variables|Default|GetMeshComponent) "NoCollision")
  (Components|StaticMesh|SetStaticMesh (Variables|Default|GetMeshComponent) "/Game/Mods/ModdingFramework_P/Meshes/ST_Megaphone1.ST_Megaphone1")
  (Transformation|AttachActorToActor (Variables|Default|GetSpawnedActor) (Variables|Default|GetOverlapped%20Actor) "None" "SnapToTarget" "SnapToTarget" "KeepRelative" true))

(event EventBeginPlay
  (Development|SetHiddeninGame (Variables|Default|GetPlane) true false))

(fn ConstructionScript)