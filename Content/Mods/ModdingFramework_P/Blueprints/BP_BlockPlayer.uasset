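; BP_BlockPlayer is a modding framework actor that changes the player pawn's collision type inside a sphere zone, apparently to block its movement.
; When a component named like "cylinder" begins overlapping the sphere, all matching capsules on that BP_Pawn switch to the Vehicle object type.
; End overlap restores them to Pawn, with wildcard display-name matching selecting the capsules.
; Both plane components are hidden at BeginPlay.
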(event OnComponentBeginOverlap(Sphere)
  (params (OverlappedComponent :type Primitive%20Component%20Object%20Reference) (OtherActor :type Actor%20Object%20Reference) (OtherComp :type Primitive%20Component%20Object%20Reference) (OtherBodyIndex :type Integer) (bFromSweep :type Boolean) (SweepResult :type Hit%20Result%20Structure%20%28by%20ref%29))
  (if (Class|KismetStringLibrary|MatchesWildcard (Utilities|GetDisplayName OtherComp) "*cylinder*" "IgnoreCase")
    (bind _asbp_pawn (Utilities|Casting|CastToBP_Pawn OtherActor))
    (for _array_element (Actor|GetComponentsByClass _asbp_pawn "/Script/Engine.CapsuleComponent")
      (if (Class|KismetStringLibrary|MatchesWildcard (Utilities|GetDisplayName _array_element) "*cylinder*" "IgnoreCase")
        (Collision|SetCollisionObjectType _array_element "ECC_Vehicle")))))

(event OnComponentEndOverlap(Sphere)
  (params (OverlappedComponent :type Primitive%20Component%20Object%20Reference) (OtherActor :type Actor%20Object%20Reference) (OtherComp :type Primitive%20Component%20Object%20Reference) (OtherBodyIndex :type Integer))
  (if (Class|KismetStringLibrary|MatchesWildcard (Utilities|GetDisplayName OtherComp) "*cylinder*" "IgnoreCase")
    (bind _asbp_pawn (Utilities|Casting|CastToBP_Pawn OtherActor))
    (for _array_element (Actor|GetComponentsByClass _asbp_pawn "/Script/Engine.CapsuleComponent")
      (if (Class|KismetStringLibrary|MatchesWildcard (Utilities|GetDisplayName _array_element) "*cylinder*" "IgnoreCase")
        (Collision|SetCollisionObjectType _array_element "ECC_Pawn")))))

(event EventBeginPlay
  (Development|SetHiddeninGame (Variables|Default|GetPlane) true false)
  (Development|SetHiddeninGame (Variables|Default|GetPlane1) true false))

(fn ConstructionScript)