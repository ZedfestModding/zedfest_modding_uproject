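; BP_TeleportAllPlayers is a trigger actor that teleports every BP_Pawn to the world origin when anything overlaps its Plane.
; The Plane is hidden in game at BeginPlay and its overlap event loops over all pawns.
; A failed teleport retries with a growing diagonal XY offset, which carries over to later pawns and has no attempt limit.
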(event OnComponentBeginOverlap(Plane)
  (params (OverlappedComponent :type Primitive%20Component%20Object%20Reference) (OtherActor :type Actor%20Object%20Reference) (OtherComp :type Primitive%20Component%20Object%20Reference) (OtherBodyIndex :type Integer) (bFromSweep :type Boolean) (SweepResult :type Hit%20Result%20Structure%20%28by%20ref%29))
  (Variables|Default|SetTeleportLocation "0, 0, 0")
  (Variables|Default|SetTeleportOffset "0, 0, 0")
  (bind _outactors (Actor|GetAllActorsOfClass "/Game/NetworkRagdollIK/Blueprints/BP_Pawn.BP_Pawn_C"))
  (for _array_element _outactors
    (bind _returnvalue (Transformation|Teleport _array_element (+ (Variables|Default|GetTeleportLocation) (Variables|Default|GetTeleportOffset)) "0, 0, 0" :!label _label))
    (if (not _returnvalue)
      (Variables|Default|SetTeleportOffset (+ "50.000000,50.000000,0.000000" (Variables|Default|GetTeleportOffset)))
      (goto _label))))

(event EventBeginPlay
  (Development|SetHiddeninGame (Variables|Default|GetPlane) true false))

(fn ConstructionScript)