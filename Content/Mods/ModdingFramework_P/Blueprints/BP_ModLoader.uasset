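; BP_ModLoader is a modding framework Blueprint that keeps a ModActor present in every level except SplashLevel.
; On Tick, it checks the level name and whether its cached ModActor reference is still valid.
; When the reference is invalid, it reuses the first ModActor found in the world, or spawns one at a fixed out-of-the-way location and caches it.
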(event EventTick
  (params (DeltaSeconds :type Float%20%28single-precision%29))
  (bind _returnvalue (Game|GetCurrentLevelName true))
  (if (not (Utilities|Enum|Equal(Enum) "SplashLevel" _returnvalue))
    (Variables|Default|GetModActor
      (:then)
      (:else
        (bind _outactors (Actor|GetAllActorsOfClass "/Game/Mods/ModdingFramework_P/ModActor.ModActor_C"))
        (if (not (Utilities|IsValid (Utilities|Array|Get(acopy) _outactors)))
          (bind _returnvalue_2 (Game|SpawnActorfromClass "/Game/Mods/ModdingFramework_P/ModActor.ModActor_C" (Math|Transform|MakeTransform "999.000000,999.000000,999.000000" "0, 0, 0" "1,1,1") "AdjustIfPossibleButAlwaysSpawn" 0 0))
          (Variables|Default|SetModActor _returnvalue_2)
          (else
            (Variables|Default|SetModActor (Utilities|Array|Get(acopy) _outactors))))))))

(fn ConstructionScript)