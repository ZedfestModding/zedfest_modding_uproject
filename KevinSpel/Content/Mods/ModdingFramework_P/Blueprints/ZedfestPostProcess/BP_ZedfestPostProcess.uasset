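; Mod actor that applies Zedfest post-processing by borrowing PostProcessVolumes from Level_Demonstration, hiding setup behind a fade widget.
; Tick steps through loading PhysicsVolumeLevel, recording its CustomVolume actors with collision disabled, then instancing Level_Demonstration far below the world.
; Actor snapshots taken before each load identify new arrivals, so everything except post-process volumes and pre-existing actors is destroyed before the fade lifts.
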(event Custom|EnableZedfestPostProcess
  (if (not (Variables|Default|GetbZedfestPostProcessEnabled))
    (Variables|Default|GetPhysicsVolumeLevel
      (:then
        (if (Class|LevelStreaming|IsLevelLoaded (Variables|Default|GetPhysicsVolumeLevel))
          (if (== 0 (Utilities|Map|Length (Variables|Default|GetPhysicsVolume_InUse)))
            (CallFunction|TrimNewerActorList)
            (else
              (Variables|Default|GetLevelOR
                (:then
                  (CallFunction|DeleteExtrasfromPostProcessLevel))
                (:else
                  (CallFunction|LoadPostProcessLevel)))))))
      (:else
        (CallFunction|LoadPhysicsVolumeLevel)))))

(event Custom|FadeOn
  (bind _outactors (Actor|GetAllActorsOfClass "/Script/Engine.PlayerController"))
  (for _array_element _outactors
    (Variables|/Script/Engine.PlayerController|SetbShowMouseCursor _array_element false))
  (bind _outactors_2 (Actor|GetAllActorsOfClass "/Game/NetworkRagdollIK/Blueprints/BP_Pawn.BP_Pawn_C"))
  (for (_ _array_index) _outactors_2
    (bind _returnvalue (UserInterface|CreateWidget "/Game/Mods/ModdingFramework_P/Blueprints/ZedfestPostProcess/WBP_Fade.WBP_Fade_C" (Game|GetPlayerController _array_index)))
    (UserInterface|Viewport|AddtoViewport _returnvalue 999999)))

(event Custom|LoadPhysicsVolumeLevel
  (bind _outactors (Actor|GetAllActorsOfClass "/Script/Engine.Actor"))
  (Variables|Default|SetActorList _outactors)
  (bind _returnvalue (Class|LevelStreamingDynamic|LoadLevelInstance "PhysicsVolumeLevel" "0, 0, 0" "0, 0, 0"))
  (Variables|Default|SetPhysicsVolumeLevel _returnvalue))

(event Custom|FadeOff
  (bind _outactors (Actor|GetAllActorsOfClass "/Script/Engine.PlayerController"))
  (for _array_element _outactors
    (Variables|/Script/Engine.PlayerController|SetbShowMouseCursor _array_element true))
  (bind _foundwidgets (Widget|GetAllWidgetsOfClass "/Game/Mods/ModdingFramework_P/Blueprints/ZedfestPostProcess/WBP_Fade.WBP_Fade_C" true))
  (for _array_element_2 _foundwidgets
    (Widget|RemovefromParent _array_element_2)))

(event Custom|PrintToModLoader
  (params (Message :type String)))

(event Custom|Make_PhysicsVolume_InUse_Map
  (for _array_element (Variables|Default|GetNewerActorList)
    (Variables|Default|SetNewerActor _array_element)
    (Collision|SetActorEnableCollision (Variables|Default|GetNewerActor) false)
    (if (Class|KismetStringLibrary|MatchesWildcard (Utilities|GetDisplayName (Variables|Default|GetNewerActor)) "*CustomVolume*" "IgnoreCase")
      (Utilities|Map|Add (Variables|Default|GetPhysicsVolume_InUse) (Variables|Default|GetNewerActor) false))))

(event Custom|TrimNewerActorList
  (bind _outactors (Actor|GetAllActorsOfClass "/Script/Engine.Actor"))
  (Variables|Default|SetNewerActorList _outactors)
  (bind _arrayelement (Utilities|Array|ReverseforEachLoop (Variables|Default|GetNewerActorList))
    (:LoopBody
      (Variables|Default|SetNewerActor _arrayelement)
      (if (Utilities|Array|ContainsItem (Variables|Default|GetActorList) (Variables|Default|GetNewerActor))
        (Utilities|Array|RemoveItem (Variables|Default|GetNewerActorList) (Variables|Default|GetNewerActor))))
    (:Completed
      (CallFunction|MakePhysicsVolumeinUseMap))))

(event Custom|DeleteExtrasFromPostProcessLevel
  (if (Class|LevelStreaming|IsLevelLoaded (Variables|Default|GetLevelOR))
    (Utilities|FlowControl|Delay 0.2)
    (bind _outactors (Actor|GetAllActorsOfClass "/Script/Engine.PostProcessVolume"))
    (Utilities|Array|AppendArray (Variables|Default|GetActorList) _outactors)
    (bind _outactors_2 (Actor|GetAllActorsOfClass "/Script/Engine.Actor"))
    (for _array_element _outactors_2
      (if (not (Utilities|Array|ContainsItem (Variables|Default|GetActorList) _array_element))
        (Actor|DestroyActor _array_element)))
    (Variables|Default|SetbZedfestPostProcessEnabled true)
    (CallFunction|FadeOff)))

(event Custom|LoadPostProcessLevel
  (if (Variables|Default|GetbInitalDelayFinished)
    (bind _outactors (Actor|GetAllActorsOfClass "/Script/Engine.Actor"))
    (Variables|Default|SetActorList _outactors)
    (bind _returnvalue (Class|LevelStreamingDynamic|LoadLevelInstance "Level_Demonstration" "0.000000,0.000000,-999999.000000" "0, 0, 0"))
    (Variables|Default|SetLevelOR _returnvalue)))

(event EventBeginPlay
  (CallFunction|Fadeon)
  (Development|SetHiddeninGame (Variables|Default|GetPlane) true false)
  (if (not (Variables|Default|GetbInitalDelayFinished))
    (Utilities|FlowControl|Delay 1.0)
    (Variables|Default|SetbInitalDelayFinished true)))

(event EventTick
  (params (DeltaSeconds :type Float%20%28single-precision%29))
  (CallFunction|EnableZedfestPostProcess))

(fn ConstructionScript)