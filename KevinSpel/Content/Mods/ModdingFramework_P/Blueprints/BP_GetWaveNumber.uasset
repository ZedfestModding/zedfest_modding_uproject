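; BP_GetWaveNumber is a modding framework actor that displays the current wave number in the world on a text render component.
; BeginPlay unhides its Plane component.
; Each Tick it updates the text from BP_WaveCounter's CurrentWaveNumber, looking up and caching the first such actor whenever its reference is invalid.
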(event Custom|PrintToModLoader
  (params (Message :type String)))

(event Custom|PreBeginPlay)

(event Custom|PostBeginPlay)

(event EventBeginPlay
  (Development|SetHiddeninGame (Variables|Default|GetPlane) false false))

(event EventTick
  (params (DeltaSeconds :type Float%20%28single-precision%29))
  (Variables|Default|GetWaveCounter
    (:then
      _)
    (:else
      (bind _outactors (Actor|GetAllActorsOfClass "/Game/Mods/ModdingFramework_P/Blueprints/BP_WaveCounter.BP_WaveCounter_C"))
      (Variables|Default|SetWaveCounter (Utilities|Array|Get(acopy) _outactors))))
  (Rendering|Components|TextRender|SetText (Variables|Default|GetTextRender1) (Utilities|Text|ToText(String) (Utilities|String|ToString(Integer) (Variables|/Game/Mods/ModdingFramework_P/Blueprints/BP_WaveCounter.BP_WaveCounter_C|GetCurrentWaveNumber (Variables|Default|GetWaveCounter))))))

(fn ConstructionScript)