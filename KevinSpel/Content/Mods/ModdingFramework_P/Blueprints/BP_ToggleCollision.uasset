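; BP_ToggleCollision is a modding framework Blueprint that switches collision on a plane on and off over time.
; BeginPlay hides the plane in game.
; Tick runs through a Delay into a FlipFlop, which alternates the plane between no collision and query-and-physics every few seconds.
; Each switch updates a TextRender label to show whether collision is enabled or disabled.
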(event EventBeginPlay
  (Development|SetHiddeninGame (Variables|Default|GetPlane) true false))

(event EventTick
  (params (DeltaSeconds :type Float%20%28single-precision%29))
  (Utilities|FlowControl|Delay 5.0)
  (Utilities|FlowControl|FlipFlop
    (:A
      (Collision|SetCollisionEnabled (Variables|Default|GetPlane) "NoCollision")
      (Rendering|Components|TextRender|SetText (Variables|Default|GetTextRender) (Utilities|Text|MakeLiteralText "Collision Disabled")))
    (:B
      (Collision|SetCollisionEnabled (Variables|Default|GetPlane) "QueryAndPhysics")
      (Rendering|Components|TextRender|SetText (Variables|Default|GetTextRender) (Utilities|Text|MakeLiteralText "Collision Enabled")))))

(fn ConstructionScript)