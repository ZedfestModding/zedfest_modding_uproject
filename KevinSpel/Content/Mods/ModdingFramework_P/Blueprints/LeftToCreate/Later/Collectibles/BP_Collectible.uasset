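; Collectible actor for the modding framework, so far only a stub with debug logging and no pickup logic.
; Its construction script copies the collectable mesh from the first BP_MainMapActor found and sets the mesh to overlap all collision channels.
; Cursor-over, view-target and component-hit events send messages or object names to PrintToModLoader, an event with an empty body here.
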(event OnBeginCursorOver(StaticMesh)
  (params (TouchedComponent :type Primitive%20Component%20Object%20Reference))
  (CallFunction|PrinttoModLoader "Your Cursor Just Went Over The Collectable!"))

(event OnComponentHit(StaticMesh)
  (params (HitComponent :type Primitive%20Component%20Object%20Reference) (OtherActor :type Actor%20Object%20Reference) (OtherComp :type Primitive%20Component%20Object%20Reference) (NormalImpulse :type Vector :default "0, 0, 0") (Hit :type Hit%20Result%20Structure%20%28by%20ref%29))
  (CallFunction|PrinttoModLoader (Utilities|GetDisplayName HitComponent))
  (CallFunction|PrinttoModLoader (Utilities|GetDisplayName OtherActor))
  (CallFunction|PrinttoModLoader (Utilities|GetDisplayName OtherComp)))

(event Custom|PrintToModLoader
  (params (Message :type String)))

(event EventOnBecomeViewTarget
  (params (PC :type Player%20Controller%20Object%20Reference))
  (CallFunction|PrinttoModLoader "A Collectable is currently a viewtarget"))

(fn ConstructionScript
  (bind _outactors (Actor|GetAllActorsOfClass "/Game/Mods/ModdingFramework_P/Blueprints/MainMapActor/BP_MainMapActor.BP_MainMapActor_C"))
  (Variables|Default|SetMainMapActor (Utilities|Array|Get(acopy) _outactors))
  (Variables|Default|SetCollectableMesh (Variables|/Game/Mods/ModdingFramework_P/Blueprints/MainMapActor/BP_MainMapActor.BP_MainMapActor_C|GetCollectableMesh (Variables|Default|GetMainMapActor)))
  (Components|StaticMesh|SetStaticMesh (Variables|Default|GetStaticMesh) (Variables|/Game/Mods/ModdingFramework_P/Blueprints/MainMapActor/BP_MainMapActor.BP_MainMapActor_C|GetCollectableMesh (Variables|Default|GetMainMapActor)))
  (Collision|SetCollisionResponsetoAllChannels (Variables|Default|GetStaticMesh) "ECR_Overlap"))