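; BP_GetAllPlayers is a trigger actor that gathers every BP_Pawn in the level at its Plane when something overlaps it.
; The Plane is hidden at BeginPlay and serves as the overlap trigger, with no filter on the overlapping actor.
; Each pawn is teleported to the Plane's location plus LocationOffset, which grows diagonally per pawn to space them apart and is never reset between overlaps.
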(event OnComponentBeginOverlap(Plane)
  (params (OverlappedComponent :type Primitive%20Component%20Object%20Reference) (OtherActor :type Actor%20Object%20Reference) (OtherComp :type Primitive%20Component%20Object%20Reference) (OtherBodyIndex :type Integer) (bFromSweep :type Boolean) (SweepResult :type Hit%20Result%20Structure%20%28by%20ref%29))
  (bind _outactors (Actor|GetAllActorsOfClass "/Game/NetworkRagdollIK/Blueprints/BP_Pawn.BP_Pawn_C"))
  (for _array_element _outactors
    (Transformation|SetActorLocation _array_element (+ (Transformation|GetWorldLocation OverlappedComponent) (Variables|Default|GetLocationOffset)) false true)
    (Variables|Default|SetLocationOffset (+ "100.000000,100.000000,100.000000" (Variables|Default|GetLocationOffset)))))

(event EventBeginPlay
  (Development|SetHiddeninGame (Variables|Default|GetPlane) true false))

(fn ConstructionScript)