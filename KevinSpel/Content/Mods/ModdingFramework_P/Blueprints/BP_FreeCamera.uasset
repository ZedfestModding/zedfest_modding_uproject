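; Free-fly camera in the ModdingFramework mod, flown with WASD for horizontal directions, E and Q for up and down, and the mouse for look.
; Tick polls player controller 0 for key presses and releases, setting movement flags that Movement turns into MoveDirection calls.
; Each call combines an angle offset with the actor's rotation and steps a fixed distance per frame, without sweep or delta-time scaling.
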(event Custom|Movement
  (if (Variables|Default|GetbMoveUp)
    (CallFunction|MoveUp))
  (if (Variables|Default|GetbMoveDown)
    (CallFunction|MoveDown))
  (if (Variables|Default|GetbMoveLeft)
    (CallFunction|MoveLeft))
  (if (Variables|Default|GetbMoveRight)
    (CallFunction|MoveRight))
  (if (Variables|Default|GetbMoveForward)
    (CallFunction|MoveForward))
  (if (Variables|Default|GetbMoveBack)
    (CallFunction|MoveBack)))

(event Custom|MoveLeft
  (CallFunction|MoveDirection "0,270.000000, 0"))

(event Custom|MoveRight
  (CallFunction|MoveDirection "0,90.000000, 0"))

(event Custom|MoveBack
  (CallFunction|MoveDirection "0,180.000000, 0"))

(event Custom|MoveForward
  (CallFunction|MoveDirection "0, 0, 0"))

(event Custom|MoveUp
  (CallFunction|MoveDirection "-90.000000, 0, 0"))

(event Custom|MoveDown
  (CallFunction|MoveDirection "90.000000,0.000000, 0"))

(event Custom|MoveDirection
  (params (InputAngleDirection :type Rotator))
  (Variables|Default|SetAngleDirection InputAngleDirection)
  (Variables|Default|SetStartLocation (Transformation|GetActorLocation))
  (Variables|Default|SetEndLocation (+ (Variables|Default|GetStartLocation) (* (Math|Vector|GetForwardVector (Math|Rotator|CombineRotators (Variables|Default|GetAngleDirection) (Transformation|GetActorRotation))) 24)))
  (Transformation|SetActorRelativeLocation (Variables|Default|GetEndLocation)))

(event EventTick
  (params (DeltaSeconds :type Float%20%28single-precision%29))
  (CallFunction|Movement)
  (if (Game|Player|WasInputKeyJustPressed (Game|GetPlayerController 0) "W")
    (Variables|Default|SetbMoveForward true))
  (if (Class|PlayerController|WasInputKeyJustReleased (Game|GetPlayerController 0) "W")
    (Variables|Default|SetbMoveForward false))
  (if (Game|Player|WasInputKeyJustPressed (Game|GetPlayerController 0) "S")
    (Variables|Default|SetbMoveBack true))
  (if (Class|PlayerController|WasInputKeyJustReleased (Game|GetPlayerController 0) "S")
    (Variables|Default|SetbMoveBack false))
  (if (Game|Player|WasInputKeyJustPressed (Game|GetPlayerController 0) "A")
    (Variables|Default|SetbMoveLeft true))
  (if (Class|PlayerController|WasInputKeyJustReleased (Game|GetPlayerController 0) "A")
    (Variables|Default|SetbMoveLeft false))
  (if (Game|Player|WasInputKeyJustPressed (Game|GetPlayerController 0) "D")
    (Variables|Default|SetbMoveRight true))
  (if (Class|PlayerController|WasInputKeyJustReleased (Game|GetPlayerController 0) "D")
    (Variables|Default|SetbMoveRight false))
  (if (Game|Player|WasInputKeyJustPressed (Game|GetPlayerController 0) "E")
    (Variables|Default|SetbMoveUp true))
  (if (Class|PlayerController|WasInputKeyJustReleased (Game|GetPlayerController 0) "E")
    (Variables|Default|SetbMoveUp false))
  (if (Game|Player|WasInputKeyJustPressed (Game|GetPlayerController 0) "Q")
    (Variables|Default|SetbMoveDown true))
  (if (Class|PlayerController|WasInputKeyJustReleased (Game|GetPlayerController 0) "Q")
    (Variables|Default|SetbMoveDown false)))

(event Input|MouseEvents|MouseX
  (params (AxisValue :type Float%20%28single-precision%29))
  (Class|PlayerController|AddYawInput (Game|GetPlayerController 0) AxisValue))

(event Input|MouseEvents|MouseY
  (params (AxisValue :type Float%20%28single-precision%29))
  (bind _result (Math|Float|NegateFloat AxisValue)
    (:%20%20
      (Class|PlayerController|AddPitchInput (Game|GetPlayerController 0) _result))))

(fn ConstructionScript)