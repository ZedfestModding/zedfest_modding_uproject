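; BP_OutOfBounds is an out-of-bounds volume that returns stray player pawns and NPCs to a player start.
; When an actor begins overlapping its Box, it checks for a BP_NPC_Base or BP_Pawn and ignores anything else.
; Matching actors are teleported without sweep to slightly above a randomly indexed PlayerStart, gathered on each overlap.
; The random index range includes the array length, so it can land one past the last start.
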(event OnComponentBeginOverlap(Box)
  (params (OverlappedComponent :type Primitive%20Component%20Object%20Reference) (OtherActor :type Actor%20Object%20Reference) (OtherComp :type Primitive%20Component%20Object%20Reference) (OtherBodyIndex :type Integer) (bFromSweep :type Boolean) (SweepResult :type Hit%20Result%20Structure%20%28by%20ref%29))
  (Variables|Default|SetOverlappedActor OtherActor)
  (Utilities|Casting|CastToBP_NPC_Base (Variables|Default|GetOverlappedActor)
    (:then
      _)
    (:CastFailed
      (Utilities|Casting|CastToBP_Pawn (Variables|Default|GetOverlappedActor))))
  (bind _outactors (Actor|GetAllActorsOfClass "/Script/Engine.PlayerStart"))
  ;[1 0 0.2578] Move Player Pawn To Random Player Start
  (Transformation|SetActorLocation (Variables|Default|GetOverlappedActor) (+ (Transformation|GetActorLocation (Utilities|Array|Get(acopy) _outactors (Math|Random|RandomIntegerinRange 0 (Utilities|Array|Length _outactors)))) "0, 0,50.000000") false true))

(fn ConstructionScript)