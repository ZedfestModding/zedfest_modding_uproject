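; Trigger actor that flips visibility of its Plane and of any actor overlapping it.
; The Plane starts hidden in game on BeginPlay.
; Both begin and end overlap events call ToggleHidden, which inverts the hidden state of the overlapped Plane component and the other actor.
; States are toggled rather than set, so simultaneous overlaps flip the Plane repeatedly.
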(event OnComponentBeginOverlap(Plane)
  (params (OverlappedComponent :type Primitive%20Component%20Object%20Reference) (OtherActor :type Actor%20Object%20Reference) (OtherComp :type Primitive%20Component%20Object%20Reference) (OtherBodyIndex :type Integer) (bFromSweep :type Boolean) (SweepResult :type Hit%20Result%20Structure%20%28by%20ref%29))
  (Variables|Default|SetComponent OverlappedComponent)
  (Variables|Default|SetActor OtherActor)
  (CallFunction|ToggleHidden))

(event OnComponentEndOverlap(Plane)
  (params (OverlappedComponent :type Primitive%20Component%20Object%20Reference) (OtherActor :type Actor%20Object%20Reference) (OtherComp :type Primitive%20Component%20Object%20Reference) (OtherBodyIndex :type Integer))
  (Variables|Default|SetComponent OverlappedComponent)
  (Variables|Default|SetActor OtherActor)
  (CallFunction|ToggleHidden))

(event Custom|ToggleHidden
  (bind _actor (Variables|Default|GetActor))
  (bind _component (Variables|Default|GetComponent))
  (Development|SetHiddeninGame _component (not (Variables|/Script/Engine.SceneComponent|GetbHiddenInGame _component)) false)
  (Rendering|SetActorHiddenInGame _actor (not (Variables|/Script/Engine.Actor|GetbHidden _actor))))

(event EventBeginPlay
  (Development|SetHiddeninGame (Variables|Default|GetPlane) true false))

(fn ConstructionScript)