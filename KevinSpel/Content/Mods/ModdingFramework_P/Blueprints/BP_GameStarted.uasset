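; BP_GameStarted is a modding framework actor that displays whether the game has started on an in-world text render.
; It hides its Plane component on BeginPlay.
; Each Tick it casts player 0's pawn controller to BP_Base_HordeController and sets the text from its LobbyClosed flag.
; The PreBeginPlay, PostBeginPlay and PrintToModLoader events are empty stubs.
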(event Custom|PrintToModLoader
  (params (Message :type String)))

(event Custom|PreBeginPlay)

(event Custom|PostBeginPlay)

(event EventBeginPlay
  (Development|SetHiddeninGame (Variables|Default|GetPlane) true false))

(event EventTick
  (params (DeltaSeconds :type Float%20%28single-precision%29))
  (if (Variables|/Game/HordeTemplateBP/Blueprint/BP_Base_HordeController.BP_Base_HordeController_C|GetLobbyClosed? (.AsBP%20Base%20Horde%20Controller (Utilities|Casting|CastToBP_Base_HordeController (Pawn|GetController (Game|Player|GetPlayerPawn 0)))))
    (Rendering|Components|TextRender|SetText (Variables|Default|GetTextRender) (Utilities|Text|MakeLiteralText "Game Has Started"))
    (else
      (Rendering|Components|TextRender|SetText (Variables|Default|GetTextRender) (Utilities|Text|MakeLiteralText "Game Has Not Started")))))

(fn ConstructionScript)